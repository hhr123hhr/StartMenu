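; BP_BowHeroAIController is the AI controller for a bow hero character.
; On BeginPlay it sets up the BB_HeroAI blackboard with the pawn's start position as home, an idle time, and a random navigable point around that position as the first target location.
; It then runs the BT_BowHeroAI behavior tree, with no per-frame logic in the controller itself.
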(event `self.ReceiveBeginPlay`
  (bind _returnvalue (`self.K2_GetActorLocation` (`self.K2_GetPawn`)))
  (`|ExecutionSequence`
    (:`then_0`
      (`self.UseBlackboard` "/Game/AI/Hero/AI/BB_HeroAI.BB_HeroAI")
      (`BlackboardComponent.SetValueAsVector` (`self.Blackboard`) (`self.HomeLocKey`) _returnvalue)
      (`BlackboardComponent.SetValueAsFloat` (`self.Blackboard`) (`self.IdleTime`) 2.0)
      (`BlackboardComponent.SetValueAsVector` (`self.Blackboard`) (`self.TargetLocKey`) (`NavigationSystemV1.K2_GetRandomLocationInNavigableRadius` _returnvalue 1000.0 null null)))
    (:`then_1`
      (`self.RunBehaviorTree` "/Game/AI/Hero/AI/BT_BowHeroAI.BT_BowHeroAI"))))

(fn `UserConstructionScript`
  (`parent.UserConstructionScript`))