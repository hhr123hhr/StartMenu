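; BP_BasicBow is a hero AI Blueprint that handles firing arrows from a bow.
; Its ArrowSpawn event plays a small muzzle particle effect and spawns an Arrow at the hand_lBowSocket socket on SkeletalMesh1, using the actor's rotation.
; The arrow always spawns regardless of collision and is owned by this actor; the BeginPlay, overlap and Tick events are disabled stubs.
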(event `ArrowSpawn`
  (`GameplayStatics.SpawnEmitterAtLocation` "/Game/GabrielAguiarProd/ToonProjectilesVol1/Particles/Muzzles/P_Muzzle_Bullet01Lowpoly.P_Muzzle_Bullet01Lowpoly" (`SceneComponent.GetSocketLocation` (`self.SkeletalMesh1`) "hand_lBowSocket") (`self.K2_GetActorRotation`) (0.05 0.05 0.05))
  (`|SpawnActorFromClass` "/Game/AI/Hero/Arrow/Arrow.Arrow_C" (`KismetMathLibrary.MakeTransform` (`SceneComponent.GetSocketLocation` (`self.SkeletalMesh1`) "hand_lBowSocket") (`self.K2_GetActorRotation`)) "AlwaysSpawn" "OverrideRootScale" self null))

(fn `UserConstructionScript`
  (`parent.UserConstructionScript`))