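; BP_HeroAIController is the AI controller that starts the hero's behavior tree, BT_HeroAI.
; On BeginPlay it loads BB_HeroAI and seeds it with the pawn's current location as home, an idle time, and a random navigable point near the pawn as the first target.
; A Sequence node runs the behavior tree after this blackboard setup, leaving all further decisions to the tree.
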(event `self.ReceiveBeginPlay`
  (bind _returnvalue (`self.K2_GetActorLocation` (`self.K2_GetPawn`)))
  (`|ExecutionSequence`
    (:`then_0`
      (`self.UseBlackboard` "/Game/AI/Hero/BB_HeroAI.BB_HeroAI")
      (`BlackboardComponent.SetValueAsVector` (`self.Blackboard`) (`self.HomeLocKey`) _returnvalue)
      (`BlackboardComponent.SetValueAsFloat` (`self.Blackboard`) (`self.IdleTime`) 2.0)
      (`BlackboardComponent.SetValueAsVector` (`self.Blackboard`) (`self.TargetLocKey`) (`NavigationSystemV1.K2_GetRandomLocationInNavigableRadius` _returnvalue 1000.0 null null)))
    (:`then_1`
      (`self.RunBehaviorTree` "/Game/AI/Hero/BT_HeroAI.BT_HeroAI"))))

(fn `UserConstructionScript`)