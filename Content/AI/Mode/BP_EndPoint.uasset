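; BP_EndPoint is the goal actor that monsters reach, costing the player a life.
; When a BP_Monster_BASIC overlaps its Box, it decrements Life on HeroMonster_GameInstance, prints the value and destroys the monster.
; At zero life it prints GameOver, fades the camera and opens the StartMenu level after a delay.
; Otherwise it asks the GM_HeroMonster game mode to check the monster count.
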(event `self.Box.OnComponentBeginOverlap`
  (params (OverlappedComponent :type "PrimitiveComponent Object Reference") (OtherActor :type "Actor Object Reference") (OtherComp :type "PrimitiveComponent Object Reference") (OtherBodyIndex :type Integer) (bFromSweep :type Boolean) (SweepResult :type "HitResult Structure (by ref)"))
  (bind _asbp_monster_basic (cast `/Game/AI/Monster/BP_Monster_BASIC` OtherActor))
  (bind _ashero_monster_game_instance (cast `/Game/AI/HeroMonster_GameInstance` (`GameplayStatics.GetGameInstance`)))
  (bind _result (`/Engine/EditorBlueprintResources/StandardMacros.DecrementInt` (`/Game/AI/HeroMonster_GameInstance.Life` _ashero_monster_game_instance))
    (:`  `
      (`KismetSystemLibrary.PrintString` (`KismetTextLibrary.Conv_TextToString` (`|FormatText` "life : {life}" _result)))
      (`self.K2_DestroyActor` _asbp_monster_basic)
      (bind _ashero_monster_game_instance_2 (cast `/Game/AI/HeroMonster_GameInstance` (`GameplayStatics.GetGameInstance`)))
      (if (<= (`/Game/AI/HeroMonster_GameInstance.Life` _ashero_monster_game_instance_2) 0)
        (`KismetSystemLibrary.PrintString` "GameOver")
        (`PlayerCameraManager.StartCameraFade` (`GameplayStatics.GetPlayerCameraManager` 0) 0.0 1.0 2.0 (`self.GameoverFade`) false false)
        (`KismetSystemLibrary.Delay` 2.0)
        (`GameplayStatics.OpenLevel` "StartMenu")
        (else
          (bind _asgm_hero_monster (cast `/Game/AI/GM_HeroMonster` (`GameplayStatics.GetGameMode`)))
          (`/Game/AI/GM_HeroMonster.CheckMonsterCount` _asgm_hero_monster))))))

(fn `UserConstructionScript`)