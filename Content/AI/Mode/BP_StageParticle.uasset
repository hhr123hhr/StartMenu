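; BP_StageParticle is an actor that shows colored stage firework effects.
; Three seconds after BeginPlay, it assigns the P_StageFirWork template to its five particle system components and resets their relative scale to one.
; Each component then gets its own "Color" parameter: blue, near-white, green, red or magenta.
; The overlap, tick and construction script graphs are empty.
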(event `self.ReceiveBeginPlay`
  (bind _particlesystem (`self.ParticleSystem`))
  (`KismetSystemLibrary.Delay` 3.0)
  (`ParticleSystemComponent.SetTemplate` _particlesystem "/Game/GabrielAguiarProd/ToonProjectilesVol1/Particles/Muzzles/P_StageFirWork.P_StageFirWork")
  (`ParticleSystemComponent.SetTemplate` (`self.ParticleSystem2`) "/Game/GabrielAguiarProd/ToonProjectilesVol1/Particles/Muzzles/P_StageFirWork.P_StageFirWork")
  (`ParticleSystemComponent.SetTemplate` (`self.ParticleSystem3`) "/Game/GabrielAguiarProd/ToonProjectilesVol1/Particles/Muzzles/P_StageFirWork.P_StageFirWork")
  (`ParticleSystemComponent.SetTemplate` (`self.ParticleSystem4`) "/Game/GabrielAguiarProd/ToonProjectilesVol1/Particles/Muzzles/P_StageFirWork.P_StageFirWork")
  (`ParticleSystemComponent.SetTemplate` (`self.ParticleSystem1`) "/Game/GabrielAguiarProd/ToonProjectilesVol1/Particles/Muzzles/P_StageFirWork.P_StageFirWork")
  (`SceneComponent.SetRelativeScale3D` _particlesystem (1.0 1.0 1.0))
  (`SceneComponent.SetRelativeScale3D` (`self.ParticleSystem1`) (1.0 1.0 1.0))
  (`SceneComponent.SetRelativeScale3D` (`self.ParticleSystem2`) (1.0 1.0 1.0))
  (`SceneComponent.SetRelativeScale3D` (`self.ParticleSystem3`) (1.0 1.0 1.0))
  (`SceneComponent.SetRelativeScale3D` (`self.ParticleSystem4`) (1.0 1.0 1.0))
  (`ParticleSystemComponent.SetColorParameter` _particlesystem "Color" (struct :`B` 1.0 :`A` 1.0))
  (`ParticleSystemComponent.SetColorParameter` (`self.ParticleSystem1`) "Color" (struct :`R` 0.933333 :`G` 0.933333 :`B` 0.933333 :`A` 1.0))
  (`ParticleSystemComponent.SetColorParameter` (`self.ParticleSystem2`) "Color" (struct :`R` 0.072508 :`G` 1.0 :`A` 1.0))
  (`ParticleSystemComponent.SetColorParameter` (`self.ParticleSystem3`) "Color" (struct :`R` 1.0 :`G` 0.034274 :`A` 1.0))
  (`ParticleSystemComponent.SetColorParameter` (`self.ParticleSystem4`) "Color" (struct :`R` 1.0 :`B` 0.994078 :`A` 1.0)))

(fn `UserConstructionScript`)