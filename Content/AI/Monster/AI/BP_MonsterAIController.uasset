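; BP_MonsterAIController is the AI controller for monsters, handing their decision-making to a behavior tree.
; On BeginPlay it sets up the BB_MonsterAI blackboard, then runs BT_MonsterAI.
; Disconnected nodes that would seed home location, idle time and a random navigable target location in the blackboard never run.
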(event `self.ReceiveBeginPlay`
  (`|ExecutionSequence`
    (:`then_0`
      (`self.UseBlackboard` "/Game/AI/Monster/AI/BB_MonsterAI.BB_MonsterAI"))
    (:`then_1`
      (`self.RunBehaviorTree` "/Game/AI/Monster/AI/BT_MonsterAI.BT_MonsterAI"))))

(fn `UserConstructionScript`)