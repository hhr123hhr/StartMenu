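; Base monster AI character that patrols along a spline, fights heroes and shows a health-bar widget.
; SetState drives walk speed, montages and the blackboard state key across peace, chase, attack, combo-hit and death.
; Sight and aggro checks target the nearest hero, capped by its battle-monster count, while damage triggers counter-chase and an outline flash.
; Death notifies the game mode, releases the attacking hero and animates a material parameter before destruction.
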(event `self.ReceiveBeginPlay`
  ;[1 1 1] Begin Play 이벤트
  (set `self.CurrentHP` (`self.MaxHP`))
  (bind _aswidget_monster_hp (cast `/Game/AI/Monster/Widget/Widget_MonsterHP` (`WidgetComponent.GetUserWidgetObject` (`self.Widget`))))
  (`ProgressBar.SetPercent` (`/Game/AI/Monster/Widget/Widget_MonsterHP.HP` _aswidget_monster_hp) (/ (`self.CurrentHP`) 100.0))
  (`self.SetState` "NewEnumerator0")
  (set `self.Offset` (`KismetMathLibrary.RandomFloatInRange` -7.0 7.0)))

(event `self.ReceiveAnyDamage`
  (params (Damage :type "Float (single-precision)") (DamageType :type "DamageType Object Reference") (InstigatedBy :type "Controller Object Reference") (DamageCauser :type "Actor Object Reference"))
  ;[1 1 1] AnyDamage 이벤트
  (if (`|EnumInequality` (`self.CurrentState`) "NewEnumerator3")
    (`|ExecutionSequence`
      (:`then_0`
        (bind _asbp_hero_base (cast `/Game/AI/Hero/BP_HERO_BASE` DamageCauser))
        (`/Engine/EditorBlueprintResources/StandardMacros.IsValid` _asbp_hero_base
          (:`Is Valid`
            (`self.Counter` _asbp_hero_base))))
      (:`then_1`
        (set `self.CurrentHP` (- (`self.CurrentHP`) Damage))
        (bind _aswidget_monster_hp (cast `/Game/AI/Monster/Widget/Widget_MonsterHP` (`WidgetComponent.GetUserWidgetObject` (`self.Widget`))))
        (`ProgressBar.SetPercent` (`/Game/AI/Monster/Widget/Widget_MonsterHP.HP` _aswidget_monster_hp) (/ (`self.CurrentHP`) 100.0))
        (if (<= (`self.CurrentHP`) 0.0)
          (`self.SetState` "NewEnumerator3")
          (`PrimitiveComponent.SetCollisionEnabled` (`self.CapsuleComponent`) "PhysicsOnly")
          (bind _asgm_hero_monster (cast `/Game/AI/GM_HeroMonster` (`GameplayStatics.GetGameMode`)))
          (`/Game/AI/GM_HeroMonster.CheckMonsterCount` _asgm_hero_monster)
          (`|ExecutionSequence`
            (:`then_0`
              (bind _asbp_hero_base_2 (cast `/Game/AI/Hero/BP_HERO_BASE` DamageCauser))
              (`/Game/AI/Hero/BP_HERO_BASE.AggroCheck` _asbp_hero_base_2)
              (`/Game/AI/Hero/BP_HERO_BASE.RemoveBattleMonster` _asbp_hero_base_2 self))
            (:`then_1`
              (`|PlayMontage` (`self.SkeletalMesh`) (`|GetArrayItem` (`self.DieMontages`) (`KismetMathLibrary.RandomIntegerInRange` 0 3))
                (:`then`
                  (bind (_direction `_새_트랙_0`) (`Timeline|타임라인_4` :!via `PlayFromStart`)
                    (:`Update`
                      (`MeshComponent.SetScalarParameterValueOnMaterials` (`self.SkeletalMesh`) "Amount" `_새_트랙_0`))))
                (:`OnCompleted`
                  (`self.K2_DestroyActor`)))))))
      (:`then_2`
        (bind (_direction_2 `_새_트랙_0_2`) (`Timeline|타임라인_3` :!via `PlayFromStart`)
          (:`Update`
            (`MeshComponent.SetScalarParameterValueOnMaterials` (`self.SkeletalMesh`) "OutlineEmissive" `_새_트랙_0_2`))))
      (:`then_3`
        (bind _asbp_basic_sword (cast `/Game/AI/Hero/BP_BasicSword` DamageCauser))
        (`self.Counter` _asbp_basic_sword)))))

(event `Combo2_monster`
  (`self.SetState` "NewEnumerator5"))

(event `self.ReceiveTick`
  (params (DeltaSeconds :type "Float (single-precision)"))
  (bind (_returnvalue_x _returnvalue_y _returnvalue_z) (`KismetMathLibrary.BreakVector` (`self.K2_GetActorLocation`)))
  (bind _distancealongspline (`self.DistanceAlongSpline`))
  (bind _spline (`/Game/AI/Monster/Spline_Base.Spline` (`self.Spline_Ref`)))
  (bind (_returnvalue_x_2 _returnvalue_y_2) (`KismetMathLibrary.BreakVector` (`SplineComponent.GetLocationAtDistanceAlongSpline` _spline _distancealongspline "World")))
  ;[1 1 1] Tick 이벤트
  (`|ExecutionSequence`
    (:`then_1`
      (if (`|EnumEquality` (`self.CurrentState`) "NewEnumerator0")
        (`/Engine/EditorBlueprintResources/StandardMacros.IsValid` (`self.Spline_Ref`)
          (:`Is Valid`
            (set `self.DistanceAlongSpline` (+ (* (* 5.0 (`self.AxisValue`)) (`GameplayStatics.GetWorldDeltaSeconds`)) (`self.DistanceAlongSpline`)))
            (`self.K2_SetActorLocation` (`KismetMathLibrary.MakeVector` (+ (`self.Offset`) _returnvalue_x_2) (+ _returnvalue_y_2 (`self.Offset`)) _returnvalue_z))
            (`self.K2_SetActorRelativeRotation` (`SplineComponent.GetRotationAtDistanceAlongSpline` _spline _distancealongspline "World"))
            (set `self.B_PEACE_WALK` true)))
        (else
          (set `self.B_PEACE_WALK` false))))))

(event `SetState`
  (params (NewState :type "/Game/AI/Monster/BPE_MonsterState Enum" :default "NewEnumerator0"))
  (bind _returnvalue (`AIBlueprintHelperLibrary.GetBlackboard` (`self.GetController`)))
  (if (`|EnumInequality` (`self.CurrentState`) "NewEnumerator3")
    (bind _output_get (set `self.CurrentState` NewState))
    (`|ExecutionSequence`
      (:`then_0`
        (`/Engine/EditorBlueprintResources/StandardMacros.IsValid` _returnvalue
          (:`Is Valid`
            (`BlackboardComponent.SetValueAsEnum` _returnvalue (`self.StateKey`) _output_get))))
      (:`then_1`
        (switch `/Game/AI/Monster/BPE_MonsterState` (`self.CurrentState`)
          (:`NewEnumerator0`
            (set `CharacterMovementComponent.MaxWalkSpeed` 5.0 (`self.CharacterMovement`)))
          (:`NewEnumerator1`
            (set `CharacterMovementComponent.MaxWalkSpeed` 20.0 (`self.CharacterMovement`)))
          (:`NewEnumerator2`
            (set `CharacterMovementComponent.MaxWalkSpeed` 0.0 (`self.CharacterMovement`))
            (`|PlayMontage` (`self.SkeletalMesh`) (`|GetArrayItem` (`self.test`) (`KismetMathLibrary.RandomIntegerInRange` 0 2))
              (:`OnCompleted`
                (`self.AggroCheck`)
                (`self.SetState` "NewEnumerator1"))))
          (:`NewEnumerator3`
            (set `CharacterMovementComponent.MaxWalkSpeed` 0.0 (`self.CharacterMovement`))
            (`self.StopAnimMontage` null))
          (:`NewEnumerator5`
            (set `CharacterMovementComponent.MaxWalkSpeed` 0.0 (`self.CharacterMovement`))
            (`|PlayMontage` (`self.SkeletalMesh`) "/Game/TwinbladesExpansion/TwinbladesExpansion/Battle/Inplace/Combo2_Monster.Combo2_Monster")))))))

(event `self.PawnSensing.OnSeePawn`
  (params (Pawn :type "Pawn Object Reference"))
  (bind _targethero (`self.TargetHero`))
  (bind _asbp_hero_base (cast `/Game/AI/Hero/BP_HERO_BASE` Pawn)
    (:`then`
      (bind _battlemonsterarray (`/Game/AI/Hero/BP_HERO_BASE.BattleMonsterArray` _asbp_hero_base))
      (if (< (`KismetArrayLibrary.Array_Length` _battlemonsterarray) (`self.MaxBattelMonsterCount`))
        (`KismetArrayLibrary.Array_AddUnique` _battlemonsterarray self)
        (set `self.DistanceToHero` 500.0 :!label _label)
        (set `self.TargetHero` null)
        (bind _outactors (`GameplayStatics.GetAllActorsOfClass` "/Game/AI/Hero/BP_HERO_BASE.BP_HERO_BASE_C"))
        (for _array_element _outactors
          (bind _returnvalue (`KismetMathLibrary.VSize` (- (`self.K2_GetActorLocation`) (`self.K2_GetActorLocation` _array_element))))
          (if (< _returnvalue (`self.DistanceToHero`))
            (set `self.DistanceToHero` _returnvalue)
            (set `self.TargetHero` _array_element)))
        (`/Engine/EditorBlueprintResources/StandardMacros.IsValid` _targethero
          (:`Is Valid`
            (set `self.Instigator` _targethero)
            (`self.SetState` "NewEnumerator1")))))
    (:`CastFailed`
      (bind _asbp_basic_sword (cast `/Game/AI/Hero/BP_BasicSword` Pawn))
      (bind _battlemonsterarray_2 (`/Game/AI/Hero/BP_HERO_BASE.BattleMonsterArray` _asbp_basic_sword))
      (if (< (`KismetArrayLibrary.Array_Length` _battlemonsterarray_2) (`self.MaxBattelMonsterCount`))
        (`KismetArrayLibrary.Array_AddUnique` _battlemonsterarray_2 self)
        (goto _label)))))

(event `BasicAttack`
  (bind _returnvalue (`self.K2_GetActorLocation`))
  (bind _outactors (`GameplayStatics.GetAllActorsOfClass` "BP_Monster_BASE_C"))
  (bind _outhit (`KismetSystemLibrary.CapsuleTraceSingleForObjects` _returnvalue (+ _returnvalue (* (`self.GetActorForwardVector`) 6.0)) 3.0 2.0 (`|MakeArray` "ObjectTypeQuery3" :!type "EObjectTypeQuery Enum") false _outactors "None" true (struct :`G` 0.207014 :`B` 1.0 :`A` 1.0) (struct :`R` 1.0 :`B` 0.951921 :`A` 1.0)))
  (bind _asbp_hero_base (cast `/Game/AI/Hero/BP_HERO_BASE` (`.HitActor` (`GameplayStatics.BreakHitResult` _outhit))))
  (`/Engine/EditorBlueprintResources/StandardMacros.IsValid` _asbp_hero_base
    (:`Is Valid`
      (`CharacterMovementComponent.AddImpulse` (`Character.CharacterMovement` _asbp_hero_base) (* (`self.GetActorForwardVector` _asbp_hero_base) -10.0) false)
      (`GameplayStatics.ApplyDamage` _asbp_hero_base 4.0 null self))))

(event `AggroCheck`
  (bind _targethero (`self.TargetHero`))
  (set `self.DistanceToHero` 30.0)
  (set `self.TargetHero` null)
  (bind _outactors (`GameplayStatics.GetAllActorsOfClass` "/Game/AI/Hero/BP_HERO_BASE.BP_HERO_BASE_C"))
  (for _array_element _outactors
    (bind _returnvalue (`KismetMathLibrary.VSize` (- (`self.K2_GetActorLocation`) (`self.K2_GetActorLocation` _array_element))))
    (if (< _returnvalue (`self.DistanceToHero`))
      (set `self.DistanceToHero` _returnvalue)
      (set `self.TargetHero` _array_element)))
  (if (<= (`self.DistanceToHero`) 800.0)
    (`/Engine/EditorBlueprintResources/StandardMacros.IsValid` _targethero
      (:`Is Valid`
        (if (< (`KismetArrayLibrary.Array_Length` (`/Game/AI/Hero/BP_HERO_BASE.BattleMonsterArray` _targethero)) (`self.MaxBattelMonsterCount`))
          (set `self.Instigator` _targethero)
          (`self.SetState` "NewEnumerator1"))))))

(event `Combo2_Impulse`
  (`CharacterMovementComponent.AddImpulse` (`self.CharacterMovement`) (* (`self.GetActorForwardVector`) -5.0) true))

(event `Counter`
  (params (Hero :type "/Game/AI/Hero/BP_HERO_BASE Object Reference"))
  (bind _output_get (set `self.Instigator` Hero))
  (`self.SetState` "NewEnumerator1")
  (bind _asbp_hero_base (cast `/Game/AI/Hero/BP_HERO_BASE` Hero))
  (`/Engine/EditorBlueprintResources/StandardMacros.IncrementInt` (`/Game/AI/Hero/BP_HERO_BASE.BattleMonsterCount` _asbp_hero_base)
    (:`  `
      (`KismetSystemLibrary.PrintString` (`KismetSystemLibrary.GetDisplayName` _output_get)))))

(fn `UserConstructionScript`
  (`parent.UserConstructionScript`))