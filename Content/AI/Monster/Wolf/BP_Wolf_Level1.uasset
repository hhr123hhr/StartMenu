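; BP_Wolf_Level1 is the level 1 wolf monster, a child Blueprint that configures behavior inherited from its parent.
; On BeginPlay it sets MaxHP before running the parent logic, then zeroes the PawnSensing sight radius.
; The Counter event is empty, Tick and overlap events are disabled stubs, and a peripheral vision angle call is left unconnected.
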(event `self.ReceiveBeginPlay`
  (set `self.MaxHP` 30.0)
  (`parent.ReceiveBeginPlay`)
  (set `PawnSensingComponent.SightRadius` 0.0 (`self.PawnSensing`)))

(event `self.Counter`
  (params (Hero :type "/Game/AI/Hero/BP_HERO_BASE Object Reference")))

(fn `UserConstructionScript`
  (`parent.UserConstructionScript`))