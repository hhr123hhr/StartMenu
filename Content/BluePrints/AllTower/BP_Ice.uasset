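; BP_Ice is an ice projectile tied to a Tower that grows, drops and bursts on impact.
; While the tower is not ready, it scales up each tick with collision off, then marks the tower ready at target size; it self-destructs if the tower is invalid.
; Drop enables gravity; Hit spawns an impact effect, resets tower flags, destroys itself and deals ice-type radial damage that ignores heroes.
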(event `self.Drop`
  ;[1 1 1] Drop
  (`parent.Drop`)
  (`PrimitiveComponent.SetEnableGravity` (`self.Mesh`) true))

(event `self.ReceiveTick`
  (params (DeltaSeconds :type "Float (single-precision)"))
  (bind _tower (`self.Tower`))
  ;[1 1 1] 불 생성
  (`/Engine/EditorBlueprintResources/StandardMacros.IsValid` _tower
    (:`Is Valid`
      (if (not (`/Game/BluePrints/AllTower/BP_TowerBase.Ready` _tower))
        (`self.GrowUp`)))
    (:`Is Not Valid`
      (`self.K2_DestroyActor`))))

(event `self.ReceiveHit`
  (params (MyComp :type "PrimitiveComponent Object Reference") (Other :type "Actor Object Reference") (OtherComp :type "PrimitiveComponent Object Reference") (bSelfMoved :type Boolean) (HitLocation :type "Vector Structure") (HitNormal :type "Vector Structure") (NormalImpulse :type "Vector Structure") (Hit :type "HitResult Structure (by ref)"))
  (bind _tower (`self.Tower`))
  ;[1 1 1] 데미지
  (bind _outactors (`GameplayStatics.GetAllActorsOfClass` "/Game/AI/Hero/BP_HERO_BASE.BP_HERO_BASE_C"))
  (set `self.Hero_Array` _outactors)
  (`GameplayStatics.SpawnEmitterAtLocation` "/Game/Luos4elements2/Particles/Ice/Par_4E_Ice_Impact_01.Par_4E_Ice_Impact_01" HitLocation (struct) (0.15 0.15 0.15))
  (set `/Game/BluePrints/AllTower/BP_TowerBase.Make` false _tower)
  (`self.K2_DestroyActor`)
  (set `/Game/BluePrints/AllTower/BP_TowerBase.Ready` false _tower)
  (`GameplayStatics.ApplyRadialDamage` 100.0 HitLocation 300.0 "/Game/BluePrints/Tower_Magic/BP_IceType.BP_IceType_C" (`self.Hero_Array`) self (`GameplayStatics.GetPlayerController` 0) true))

(fn `GrowUp`
  (`self.SetActorEnableCollision` false)
  (`self.SetActorScale3D` (+ (`self.GetActorScale3D`) (0.001 0.001 0.001)))
  (if (== (`self.GetActorScale3D`) (0.06 0.06 0.06))
    (set `/Game/BluePrints/AllTower/BP_TowerBase.Ready` true (`self.Tower`))
    (`self.SetActorEnableCollision` true)
    (return)))

(fn `UserConstructionScript`
  (`parent.UserConstructionScript`))