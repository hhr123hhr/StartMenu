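; BP_TowerArea is a tower build spot that shows a tower selection actor while something overlaps it.
; Its StaticMesh overlap events swap the material and track AreaOverlap on entry.
; A DoOnce, entered or reset according to AreaSpawn, gates spawning the scaled-down selection actor at the area's location.
; Ending the overlap restores the glow material, clears AreaOverlap, destroys any valid selection actor and resets the gate.
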(event `self.StaticMesh.OnComponentBeginOverlap`
  (params (OverlappedComponent :type "PrimitiveComponent Object Reference") (OtherActor :type "Actor Object Reference") (OtherComp :type "PrimitiveComponent Object Reference") (OtherBodyIndex :type Integer) (bFromSweep :type Boolean) (SweepResult :type "HitResult Structure (by ref)"))
  (`PrimitiveComponent.SetMaterial` (`self.StaticMesh`) 0 "/Game/Frank_RPG_Archer/Materials/Body.Body")
  (set `self.AreaOverlap` true)
  (if (`self.AreaSpawn`)
    (goto _label :!via `Reset`)
    (else
      (`/Engine/EditorBlueprintResources/StandardMacros.DoOnce` false :!label _label
        (:`Completed`
          (bind _returnvalue (`|SpawnActorFromClass` "/Game/BluePrints/AllTower/BP_TowerSelect.BP_TowerSelect_C" (`KismetMathLibrary.MakeTransform` (+ (`self.K2_GetActorLocation`) (0.0 0.0 0.0)) (struct) (0.01 0.01 0.01)) "Undefined" "OverrideRootScale" null null)))))))

(event `self.StaticMesh.OnComponentEndOverlap`
  (params (OverlappedComponent :type "PrimitiveComponent Object Reference") (OtherActor :type "Actor Object Reference") (OtherComp :type "PrimitiveComponent Object Reference") (OtherBodyIndex :type Integer))
  (`PrimitiveComponent.SetMaterial` (`self.StaticMesh`) 0 "/Game/Frank_RPG_Archer/Materials/FX_Glow1.FX_Glow1")
  (set `self.AreaOverlap` false)
  (`/Engine/EditorBlueprintResources/StandardMacros.IsValid` (stale `self.StaticMesh.OnComponentBeginOverlap` _returnvalue)
    (:`Is Valid`
      (`self.K2_DestroyActor` (stale `self.StaticMesh.OnComponentBeginOverlap` _returnvalue))
      (goto _label :!via `Reset`))))

(fn `UserConstructionScript`)