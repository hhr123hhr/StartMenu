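; BP_TowerBase is a tower that automatically attacks monsters entering its sphere range.
; On BeginPlay it loads its stats from a data table row: attack type, damage and attack speed.
; Sphere overlaps maintain an enemy list, with a DoOnce starting a looping attack timer that stops and resets when the list empties.
; Each tick of that timer spawns an attack actor at ShootingPoint, targeting the first listed enemy.
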(event `self.ReceiveBeginPlay`
  (bind _returnvalue (`|GetDataTableRow` "/Game/HR/BP_HRDataTable.BP_HRDataTable" (`self.row`))
    (:`then`
      (set `self.Tower종류` _returnvalue))))

(event `self.Sphere1.OnComponentBeginOverlap`
  (params (OverlappedComponent :type "PrimitiveComponent Object Reference") (OtherActor :type "Actor Object Reference") (OtherComp :type "PrimitiveComponent Object Reference") (OtherBodyIndex :type Integer) (bFromSweep :type Boolean) (SweepResult :type "HitResult Structure (by ref)"))
  (bind _asbp_monster_basic (cast `/Game/AI/Monster/BP_Monster_BASIC` OtherActor))
  (`KismetArrayLibrary.Array_Add` (`self.ListOfEnemy`) _asbp_monster_basic)
  (`/Engine/EditorBlueprintResources/StandardMacros.DoOnce` false :!label _label
    (:`Completed`
      (`KismetSystemLibrary.K2_SetTimer` null "AttackEnemy1" (`.TowerAttackSpeed_18_A8719F8E4CCD328B3B8027A0E52B601F` (break `/Game/HR/BP_HRStruct` (`self.Tower종류`))) true))))

(event `self.Sphere1.OnComponentEndOverlap`
  (params (OverlappedComponent :type "PrimitiveComponent Object Reference") (OtherActor :type "Actor Object Reference") (OtherComp :type "PrimitiveComponent Object Reference") (OtherBodyIndex :type Integer))
  (bind _asbp_monster_basic (cast `/Game/AI/Monster/BP_Monster_BASIC` OtherActor))
  (`KismetArrayLibrary.Array_RemoveItem` (`self.ListOfEnemy`) _asbp_monster_basic)
  (if (== (`KismetArrayLibrary.Array_Length` (`self.ListOfEnemy`)) 0)
    (`KismetSystemLibrary.K2_ClearTimer` null "AttackEnemy1")
    (goto _label :!via `Reset`)))

(fn `AttackEnemy1`
  (locals (NewLocalVar_0 :type "/Game/HR/BP_HRBulletBase Object Reference"))
  (bind _listofenemy (`self.ListOfEnemy`))
  (bind (_towernumber _towername _towerattackspeed _towerdamage _towerange _towerselection _attacktype) (break `/Game/HR/BP_HRStruct` (`self.Tower종류`)))
  (if (!= (`KismetArrayLibrary.Array_Length` _listofenemy) 0)
    (bind _returnvalue (`|SpawnActorFromClass` _attacktype (`SceneComponent.K2_GetComponentToWorld` (`self.Shooting Point`)) "AlwaysSpawn" "OverrideRootScale" null _towerdamage null))
    (`/Engine/EditorBlueprintResources/StandardMacros.IsValid` null
      (:`Is Valid`
        (set `/Game/HR/BP_HRBulletBase.EnemyToAttack` (`|GetArrayItem` _listofenemy) _returnvalue)))))

(fn `UserConstructionScript`)