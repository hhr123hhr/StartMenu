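; BP_CancleMenu is an overlap actor, apparently the cancel option of a VR motion-controller menu.
; When the first MotionControllerPawn's right controller overlaps it, it shows that controller's Pointer, raises FireOverlap and sets the pawn's Select to the cancel index.
; Any end overlap hides the Pointer and clears FireOverlap without checking the actor or resetting Select, reusing the pawn lookup from begin overlap.
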(event `self.ReceiveActorBeginOverlap`
  (params (OtherActor :type "Actor Object Reference"))
  (bind _outactors (`GameplayStatics.GetAllActorsOfClass` "/Game/VirtualRealityBP/Blueprints/MotionControllerPawn.MotionControllerPawn_C"))
  (bind _output (`|GetArrayItem` _outactors))
  (bind _rightcontroller (`/Game/VirtualRealityBP/Blueprints/MotionControllerPawn.RightController` _output))
  (if (== OtherActor _rightcontroller)
    (`SceneComponent.SetVisibility` (`/Game/VirtualRealityBP/Blueprints/BP_MotionController.Pointer` _rightcontroller) true false)
    (set `self.FireOverlap` true)
    (set `/Game/VirtualRealityBP/Blueprints/MotionControllerPawn.Select` 3 _output)))

(event `self.ReceiveActorEndOverlap`
  (params (OtherActor :type "Actor Object Reference"))
  (`SceneComponent.SetVisibility` (`/Game/VirtualRealityBP/Blueprints/BP_MotionController.Pointer` (`/Game/VirtualRealityBP/Blueprints/MotionControllerPawn.RightController` (`|GetArrayItem` (stale `self.ReceiveActorBeginOverlap` _outactors)))) false false)
  (set `self.FireOverlap` false))

(fn `UserConstructionScript`)