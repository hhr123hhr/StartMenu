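; Ice projectile for a magic tower that grows until ready, then deals ice-type radial damage when it hits.
; Tick scales it up with collision off until it reaches half scale, then enables collision and sets the tower's Ready flag.
; Drop extends the parent event by enabling gravity.
; Hit spawns a generic explosion effect, clears the tower's Make and Ready flags, destroys the actor and applies the damage.
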(event `self.Drop`
  ;[1 1 1] Drop
  (`parent.Drop`)
  (`PrimitiveComponent.SetEnableGravity` (`self.StaticMeshComponent`) true))

(event `self.ReceiveTick`
  (params (DeltaSeconds :type "Float (single-precision)"))
  ;[1 1 1] 불 생성
  (if (not (`/Game/BluePrints/Tower_Magic/BP_IceTower.Ready` (`self.Tower`)))
    (`self.GrowUp`)))

(event `self.ReceiveHit`
  (params (MyComp :type "PrimitiveComponent Object Reference") (Other :type "Actor Object Reference") (OtherComp :type "PrimitiveComponent Object Reference") (bSelfMoved :type Boolean) (HitLocation :type "Vector Structure") (HitNormal :type "Vector Structure") (NormalImpulse :type "Vector Structure") (Hit :type "HitResult Structure (by ref)"))
  (bind _tower (`self.Tower`))
  ;[1 1 1] 불 파괴
  (`|SpawnActorFromClass` "/Game/StarterContent/Blueprints/Blueprint_Effect_Explosion.Blueprint_Effect_Explosion_C" (`KismetMathLibrary.MakeTransform` HitLocation) "Undefined" "OverrideRootScale" null null) ; 얼음이펙트로 변경
  (set `/Game/BluePrints/Tower_Magic/BP_IceTower.Make` false _tower)
  (`self.K2_DestroyActor`)
  (set `/Game/BluePrints/Tower_Magic/BP_IceTower.Ready` false _tower)
  (`GameplayStatics.ApplyRadialDamage` :`BaseDamage` 300.0 :`Origin` HitLocation :`DamageRadius` 300.0 :`DamageTypeClass` "/Game/BluePrints/Tower_Magic/BP_IceType.BP_IceType_C" :`DamageCauser` null :`InstigatedByController` null :`bDoFullDamage` true :`DamagePreventionChannel` "ECC_Destructible"))

(fn `GrowUp`
  (`self.SetActorEnableCollision` false)
  (`self.SetActorScale3D` (+ (`self.GetActorScale3D`) (0.001 0.001 0.001)))
  (if (== (`self.GetActorScale3D`) (0.5 0.5 0.5))
    (set `/Game/BluePrints/Tower_Magic/BP_IceTower.Ready` true (`self.Tower`))
    (`self.SetActorEnableCollision` true)
    (return)))

(fn `UserConstructionScript`
  (`parent.UserConstructionScript`))