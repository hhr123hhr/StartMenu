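; Ice tower actor that spawns a small BP_Ice actor above itself.
; Tick checks a Make flag cleared on BeginPlay, waits one second, spawns BP_Ice with itself as Tower, then sets Make.
; Nothing here clears the flag again after a spawn.
; Unconnected leftover nodes hold a variant that keeps the flag on the GameInstance and spawns BP_Fire.
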(event `self.ReceiveTick`
  (params (DeltaSeconds :type "Float (single-precision)"))
  (if (not (`self.Make`))
    (`KismetSystemLibrary.Delay` 1.0)
    (`|SpawnActorFromClass` "/Game/BluePrints/Tower_Magic/BP_Ice.BP_Ice_C" (`KismetMathLibrary.MakeTransform` (+ (`self.K2_GetActorLocation`) (0.0 0.0 90.0)) (struct) (0.1 0.1 0.1)) "Undefined" "OverrideRootScale" null self null)
    (set `self.Make` true)))

(event `self.ReceiveBeginPlay`
  (set `self.Make` false))

(fn `UserConstructionScript`)