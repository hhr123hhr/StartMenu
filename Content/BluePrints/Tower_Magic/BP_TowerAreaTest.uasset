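; BP_TowerAreaTest is a test area actor for the magic tower that reacts to the player's right VR motion controller.
; When that controller begins overlapping, it shows the controller's pointer, swaps the mesh to a blue debug material and sets an AreaOverlap flag.
; Any end overlap reverses all three without checking the actor, reusing the pawn lookup from begin overlap.
; BeginPlay also stores the actor's location.
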(event `self.ReceiveBeginPlay`
  (set `self.Location` (`self.K2_GetActorLocation`)))

(event `self.ReceiveActorBeginOverlap`
  (params (OtherActor :type "Actor Object Reference"))
  (bind _outactors (`GameplayStatics.GetAllActorsOfClass` "/Game/VirtualRealityBP/Blueprints/MotionControllerPawn.MotionControllerPawn_C"))
  (bind _rightcontroller (`/Game/VirtualRealityBP/Blueprints/MotionControllerPawn.RightController` (`|GetArrayItem` _outactors)))
  (if (== OtherActor _rightcontroller)
    (`SceneComponent.SetVisibility` (`/Game/VirtualRealityBP/Blueprints/BP_MotionController.Pointer` _rightcontroller) true false)
    (`PrimitiveComponent.SetMaterial` (`self.StaticMesh`) 0 "/Engine/EngineDebugMaterials/VertexColorViewMode_BlueOnly.VertexColorViewMode_BlueOnly")
    (set `self.AreaOverlap` true)))

(event `self.ReceiveActorEndOverlap`
  (params (OtherActor :type "Actor Object Reference"))
  (`SceneComponent.SetVisibility` (`/Game/VirtualRealityBP/Blueprints/BP_MotionController.Pointer` (`/Game/VirtualRealityBP/Blueprints/MotionControllerPawn.RightController` (`|GetArrayItem` (stale `self.ReceiveActorBeginOverlap` _outactors)))) false false)
  (`PrimitiveComponent.SetMaterial` (`self.StaticMesh`) 0 "/Engine/MapTemplates/Sky/M_BlackBackground.M_BlackBackground")
  (set `self.AreaOverlap` false))

(fn `UserConstructionScript`)