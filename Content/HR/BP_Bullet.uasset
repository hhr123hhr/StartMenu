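; BP_Bullet is a homing projectile that damages monsters derived from BP_Monster_BASE.
; Each tick it moves toward EnemyToAttack at Speed by world offset without sweep, caching the target's location to head there if the target becomes invalid.
; Its Sphere overlap applies Damage to monsters and destroys the bullet on any contact; otherwise a short lifespan set at BeginPlay removes it.
; Older direct health-subtraction and enemy-destroy logic remains disconnected.
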(event `self.ReceiveBeginPlay`
  (`self.SetLifeSpan` 3.0)
  (`KismetSystemLibrary.PrintString` "Hello"))

(event `self.ReceiveTick`
  (params (DeltaSeconds :type "Float (single-precision)"))
  (bind _enemytoattack (`self.EnemyToAttack`))
  (bind _returnvalue (`self.K2_GetActorLocation` _enemytoattack))
  (`/Engine/EditorBlueprintResources/StandardMacros.IsValid` _enemytoattack
    (:`Is Valid`
      (`self.K2_AddActorWorldOffset` (* (`KismetMathLibrary.Normal` (- _returnvalue (`self.K2_GetActorLocation`))) (* DeltaSeconds (`self.Speed`))))
      (`/Engine/EditorBlueprintResources/StandardMacros.IsValid` (`self.EnemyToAttack`)
        (:`Is Valid`
          (set `self.LastLocation` _returnvalue))))
    (:`Is Not Valid`
      (`self.K2_AddActorWorldOffset` (* (`KismetMathLibrary.Normal` (- (`self.LastLocation`) (`self.K2_GetActorLocation`))) (* (`self.Speed`) DeltaSeconds)))
      (`/Engine/EditorBlueprintResources/StandardMacros.IsValid` _enemytoattack))))

(event `self.Sphere.OnComponentBeginOverlap`
  (params (OverlappedComponent :type "PrimitiveComponent Object Reference") (OtherActor :type "Actor Object Reference") (OtherComp :type "PrimitiveComponent Object Reference") (OtherBodyIndex :type Integer) (bFromSweep :type Boolean) (SweepResult :type "HitResult Structure (by ref)"))
  (bind _asbp_monster_base (cast `/Game/VirtualRealityBP/Blueprints/BP_Monster_BASE` OtherActor)
    (:`then`
      (`GameplayStatics.ApplyDamage` _asbp_monster_base (`self.Damage`))
      (`self.K2_DestroyActor`))
    (:`CastFailed`
      (`self.K2_DestroyActor`))))

(fn `UserConstructionScript`)